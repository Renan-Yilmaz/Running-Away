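; Player character for parkour movement, with sprint, double jump, crouch, slide, wall run and ladder climb.
; Timelines drive sprint speed, a swept slide that halves the capsule, FOV kicks and camera roll on slides and side-wall contact.
; WallDetect overlaps reset the double jump and, on tagged surfaces with Space held, suspend gravity, constrain the movement plane and push along camera forward.
; Tick plays walk or sprint camera shakes; BeginPlay stores the start location as CheckPoint.
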(event EventBeginPlay
  (Variables|Default|SetCheckPoint (Transformation|GetActorLocation)))

(event EventTick
  (params (DeltaSeconds :type Float%20%28single-precision%29))
  (CallFunction|CheckShake))

(fn ConstructionScript)

(event OnComponentBeginOverlap(WallRight)
  (params (OverlappedComponent :type Primitive%20Component%20Object%20Reference) (OtherActor :type Actor%20Object%20Reference) (OtherComp :type Primitive%20Component%20Object%20Reference) (OtherBodyIndex :type Integer) (bFromSweep :type Boolean) (SweepResult :type Hit%20Result%20Structure%20%28by%20ref%29))
  ;[1 1 1] Rotate Wall Ride
  (if (Utilities|CheckWallRide OtherComp)
    (bind _alpha (Timeline|SmoothRotateRight PlayFromStart)
      (:Update
        (Pawn|SetControlRotation (Game|GetPlayerController 0) (|Rotation-20 _alpha))))))

(event OnComponentBeginOverlap(WallLeft)
  (params (OverlappedComponent :type Primitive%20Component%20Object%20Reference) (OtherActor :type Actor%20Object%20Reference) (OtherComp :type Primitive%20Component%20Object%20Reference) (OtherBodyIndex :type Integer) (bFromSweep :type Boolean) (SweepResult :type Hit%20Result%20Structure%20%28by%20ref%29))
  ;[1 1 1] Rotate Wall Ride
  (if (Utilities|CheckWallRide OtherComp)
    (bind _alpha (Timeline|SmoothRotateLeft PlayFromStart)
      (:Update
        (Pawn|SetControlRotation (Game|GetPlayerController 0) (|Rotation+20 _alpha))))))

(event OnComponentEndOverlap(WallRight)
  (params (OverlappedComponent :type Primitive%20Component%20Object%20Reference) (OtherActor :type Actor%20Object%20Reference) (OtherComp :type Primitive%20Component%20Object%20Reference) (OtherBodyIndex :type Integer))
  ;[1 1 1] End Overlap wall ride (left/right)
  (if (Utilities|CheckWallRide OtherComp)
    (Utilities|String|Reverse (Variables|Default|GetSmoothRotateRight))))

(event OnComponentEndOverlap(WallLeft)
  (params (OverlappedComponent :type Primitive%20Component%20Object%20Reference) (OtherActor :type Actor%20Object%20Reference) (OtherComp :type Primitive%20Component%20Object%20Reference) (OtherBodyIndex :type Integer))
  ;[1 1 1] End Overlap wall ride (left/right)
  (if (Utilities|CheckWallRide OtherComp)
    (Utilities|String|Reverse (Variables|Default|GetSmoothRotateLeft))))

(event OnComponentBeginOverlap(WallDetect)
  (params (OverlappedComponent :type Primitive%20Component%20Object%20Reference) (OtherActor :type Actor%20Object%20Reference) (OtherComp :type Primitive%20Component%20Object%20Reference) (OtherBodyIndex :type Integer) (bFromSweep :type Boolean) (SweepResult :type Hit%20Result%20Structure%20%28by%20ref%29))
  (bind _charactermovement (Variables|Character|GetCharacterMovement))
  (bind _charactermovement_2 (Variables|Character|GetCharacterMovement))
  ;[1 1 1] Wall detection
  (Utilities|FlowControl|Sequence
    (:then_0
      (CallFunction|ResetDoubleJump))
    (:then_1
      (Variables|Default|SetPlayerDirection (|ForwardCamera))
      ;[1 1 1] Wall ride System
      (if (Utilities|CheckWallRide OtherComp)
        (Variables|Default|SetOnWall true)
        (Timeline|WallRun Play
          (:Update
            (if (Game|Player|IsInputKeyDown (Game|GetPlayerController 0) "SpaceBar")
              (if (Variables|Default|GetOnWall)
                (Variables|/Script/Engine.CharacterMovementComponent|SetGravityScale _charactermovement 0.0)
                (Class|MovementComponent|SetPlaneConstraintNormal _charactermovement "0, 0,1.000000")
                (Physics|AddForce (Variables|Character|GetCharacterMovement) (* (Variables|Default|GetPlayerDirection) (Variables|Default|GetWallRunSpeed)))))))
        (else
          ;[1 1 1] Ladder Climb
          (if (Components|ComponentHasTag OtherComp "Ladder")
            (Variables|Default|SetOnWall true)
            (Timeline|Ladder Play
              (:Update
                (if (Game|Player|IsInputKeyDown (Game|GetPlayerController 0) "SpaceBar")
                  (if (Variables|Default|GetOnWall)
                    (Variables|/Script/Engine.CharacterMovementComponent|SetGravityScale _charactermovement_2 0.0)
                    (Class|MovementComponent|SetPlaneConstraintNormal _charactermovement_2 "0,1.000000,0.000000")
                    (Physics|AddForce _charactermovement_2 (* (Variables|Default|GetPlayerDirection) (Variables|Default|GetLadderSpeed)))))))))))))

(event OnComponentEndOverlap(WallDetect)
  (params (OverlappedComponent :type Primitive%20Component%20Object%20Reference) (OtherActor :type Actor%20Object%20Reference) (OtherComp :type Primitive%20Component%20Object%20Reference) (OtherBodyIndex :type Integer))
  (bind _charactermovement (Variables|Character|GetCharacterMovement))
  ;[1 1 1] Stop wall ride or ladder end overlap
  (Utilities|FlowControl|Sequence
    (:then_0
      (Audio|Components|Audio|Stop (Variables|Default|GetWallRun))
      (Audio|Components|Audio|Stop (Variables|Default|GetLadder)))
    (:then_1
      (if (or (Components|ComponentHasTag OtherComp "WallRide") (Components|ComponentHasTag OtherComp "Ladder"))
        (Variables|/Script/Engine.CharacterMovementComponent|SetGravityScale _charactermovement 2.0)
        (Class|MovementComponent|SetPlaneConstraintNormal _charactermovement "0, 0, 0")
        (Variables|Default|SetOnWall false)))))

(event Custom|ResetView
  ;[1 1 1] End jump
  (bind _newtrack_0 (Timeline|Timeline_2 PlayFromStart)
    (:Update
      (Camera|SetFieldOfView (Variables|Default|GetCamera) (Math|Float|MapRangeClamped _newtrack_0 0.0 1.0 1.1e+02 9e+01)))))

(event Custom|ResetDoubleJump
  ;[1 1 1] Jump System
  ;;[1 1 1] Double jump
  (Utilities|FlowControl|DoOnce false) ; enters at Reset
)

(event Custom|CheckShake
  (bind _returnvalue (Transformation|GetActorLocation))
  ;[1 1 1] Camera shaking
  (if (Math|Boolean|ANDBoolean (Variables|Default|GetSprinting) (not (AI|Components|NavMovement|IsFalling (Variables|Character|GetCharacterMovement))) (> (Math|Vector|VectorLength (Variables|/Script/Engine.MovementComponent|GetVelocity (Variables|Character|GetCharacterMovement))) 0.0))
    (Camera|PlayWorldCameraShake "/Game/Blueprints/CameraShake/BP_CameraShakeSprint.BP_CameraShakeSprint_C" _returnvalue 0.0 5e+02)
    (elif (> (Math|Vector|VectorLength (Variables|/Script/Engine.MovementComponent|GetVelocity (Variables|Character|GetCharacterMovement))) 0.0)
      (Camera|PlayWorldCameraShake "/Game/Blueprints/CameraShake/BP_CameraShakeWalk.BP_CameraShakeWalk_C" _returnvalue 0.0 5e+02))))

(event EventOnLanded
  (params (Hit :type Hit%20Result%20Structure%20%28by%20ref%29))
  ;[1 1 1] End jump
  (Variables|Default|SetFirstJump false)
  (CallFunction|ResetDoubleJump)
  (if (Variables|Default|GetViewChanged)
    (Variables|Default|SetViewChanged false)
    (bind _newtrack_0 (Timeline|Timeline_2 PlayFromStart)
      (:Update
        (Camera|SetFieldOfView (Variables|Default|GetCamera) (Math|Float|MapRangeClamped _newtrack_0 0.0 1.0 1.1e+02 9e+01))))))

(event Input|ActionEvents|InputActionJump
  (params (Key :type Key%20Structure :default "None"))
  ;[1 1 1] Jump System
  (:Pressed
    (if (and (Variables|Default|GetFirstJump) (not (Variables|Default|GetSliding)))
      ;;[1 1 1] Double jump
      (Utilities|FlowControl|DoOnce false
        (:Completed
          (Character|LaunchCharacter "0, 0,900.000000" false true)))
      (else
        (Variables|Default|SetFirstJump true)
        (Character|Jump)
        (if (|Velocity>1100)
          (Variables|Default|SetViewChanged true)
          ;[1 1 1] Camera effect on jump
          (bind _newtrack_0 (Timeline|Timeline_1 PlayFromStart)
            (:Update
              (Camera|SetFieldOfView (Variables|Default|GetCamera) (Math|Float|MapRangeClamped _newtrack_0 0.0 1.0 9e+01 1.1e+02))))))))
  (:Released
    (Character|StopJumping)
    (Audio|Components|Audio|Stop (Variables|Default|GetWallRun))
    (Audio|Components|Audio|Stop (Variables|Default|GetLadder))
    (Variables|Default|SetOnWall false)))

(event Input|ActionEvents|InputActionCrouch/Slide
  (params (Key :type Key%20Structure :default "None"))
  (bind _returnvalue (Transformation|GetActorLocation))
  (bind _capsulecomponent (Variables|Collision|GetCapsuleComponent))
  (bind _springarm (Variables|Default|GetSpringArm))
  (bind _springarm_2 (Variables|Default|GetSpringArm))
  (bind _springarm_3 (Variables|Default|GetSpringArm))
  (bind _springarm_4 (Variables|Default|GetSpringArm))
  (bind _relativelocation (Variables|/Script/Engine.SceneComponent|GetRelativeLocation _springarm_3))
  (bind _relativelocation_2 (Variables|/Script/Engine.SceneComponent|GetRelativeLocation _springarm_4))
  (bind (_x _y _z) (Math|Vector|BreakVector _relativelocation))
  (bind (_x_2 _y_2 _z_2) (Math|Vector|BreakVector _relativelocation_2))
  (:Pressed
    (if (Variables|Default|GetSprinting)
      (if (|VelocityCheck)
        (Variables|Default|SetStartLocation _returnvalue)
        (Variables|Default|SetEndLocation (+ _returnvalue (* (Transformation|GetActorForwardVector) (Variables|Default|GetSlideDistance))))
        (bind _alpha (Timeline|Slide PlayFromStart)
          (:Update
            (Variables|Default|SetSliding true)
            (Transformation|SetActorLocation (Math|Vector|Lerp(Vector) (Variables|Default|GetStartLocation) (Variables|Default|GetEndLocation) _alpha) true false)
            (Camera|SetFieldOfView (Variables|Default|GetCamera) (Math|Float|Lerp 9e+01 1.1e+02 _alpha))
            (Pawn|SetControlRotation (Game|GetPlayerController 0) (|SlideEffect _alpha))
            (Components|Capsule|SetCapsuleHalfHeight _capsulecomponent (/ (Components|Capsule|GetScaledCapsuleHalfHeight _capsulecomponent) 2.0) true)
            (Transformation|SetRelativeLocation _springarm_2 (Math|Vector|Lerp(Vector) (Variables|/Script/Engine.SceneComponent|GetRelativeLocation _springarm_2) "0, 0, 0" _alpha) true false))
          (:Finished
            (CallFunction|ResetView)
            (Variables|Default|SetSliding false)
            (bind _alpha_2 (Timeline|Timeline_3 PlayFromStart)
              (:Update
                (Pawn|SetControlRotation (Game|GetPlayerController 0) (|ReverseSlideEffect _alpha_2)))
              (:Finished
                (Components|Capsule|SetCapsuleHalfHeight (Variables|Collision|GetCapsuleComponent) 88.0 true)
                (Transformation|SetRelativeLocation _springarm (Math|Vector|Lerp(Vector) (Variables|/Script/Engine.SceneComponent|GetRelativeLocation _springarm) "0, 0,75.000000" _alpha_2) true false))))))
      (else
        (Character|Crouch)
        (Transformation|SetRelativeLocation _springarm_4 (Math|Vector|MakeVector _x_2 _y_2 (- _z_2 18.0)) true false))))
  (:Released
    (Character|UnCrouch)
    (Transformation|SetRelativeLocation _springarm_3 (Math|Vector|MakeVector _x _y (+ _z 18.0)) true false)))

(event Input|ActionEvents|InputActionSprint
  (params (Key :type Key%20Structure :default "None"))
  ;[1 1 1] Sprint
  (:Pressed
    (Variables|Default|SetSprinting true)
    (bind _newtrack_0 (Timeline|Timeline_0 Play)
      (:Update
        _)
      (:Finished
        _))
    (Variables|/Script/Engine.CharacterMovementComponent|SetMaxWalkSpeed (Variables|Character|GetCharacterMovement) (Math|Float|Lerp 9e+02 1.5e+03 _newtrack_0)))
  (:Released
    (Variables|Default|SetSprinting false)
    (Timeline|Timeline_0 Reverse)))

(event Input|AxisEvents|InputAxisRight
  (params (AxisValue :type Float%20%28single-precision%29))
  ;[1 1 1] Basic movement
  (if (not (Variables|Default|GetOnWall))
    (Pawn|Input|AddMovementInput (.Right (|Movementcalcul)) AxisValue false)))

(event Input|AxisEvents|InputAxisForward
  (params (AxisValue :type Float%20%28single-precision%29))
  ;[1 1 1] Basic movement
  (if (not (Variables|Default|GetOnWall))
    (Pawn|Input|AddMovementInput (.Forward (|Movementcalcul)) AxisValue false)))

(event Input|AxisEvents|InputAxisTurnrate
  (params (AxisValue :type Float%20%28single-precision%29))
  ;[1 1 1] Basic movement
  (Pawn|Input|AddControllerYawInput AxisValue))

(event Input|AxisEvents|InputAxisLookUp
  (params (AxisValue :type Float%20%28single-precision%29))
  ;[1 1 1] Basic movement
  (Pawn|Input|AddControllerPitchInput AxisValue))